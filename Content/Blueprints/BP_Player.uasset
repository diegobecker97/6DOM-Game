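; BP_Player is the player Blueprint, handling death and objective-based winning.
; When its health component fires OnDeath, it shows the end screen, disables player input and opens SpaceLevel after a short delay.
; Overlapping an actor tagged Objective destroys that actor and decrements ObjectivesToVisit, adding a win screen widget to the viewport when the count reaches zero.
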(event Custom|HandlePlayerDeath
  ;[0.15 0.15 0.15 0.5] Player death
  (bind _returnvalue (UserInterface|CreateWidget "/Game/Blueprints/WBP_EndScreen.WBP_EndScreen_C"))
  (UserInterface|Viewport|AddtoViewport _returnvalue 0)
  (Input|DisableInput (Game|GetPlayerController 0) 0)
  (Utilities|FlowControl|Delay 5.0)
  (Game|OpenLevel(byObjectReference) "/Game/SpaceLevel.SpaceLevel"))

(event EventBeginPlay
  ;[0.15 0.15 0.15 0.5] Player death
  (EventDispatchers|BindEventtoOnDeath (Variables|Default|GetBP_HealthComponent) (delegate Custom|HandlePlayerDeath)))

(event Collision|EventActorBeginOverlap
  (params (OtherActor :type Actor%20Object%20Reference))
  ;[0.15 0.15 0.15 0.5] Objective
  (Utilities|IsValid OtherActor
    (:Is%20Valid
      (if (Actor|ActorHasTag OtherActor "Objective")
        (Actor|DestroyActor OtherActor)
        (Variables|Default|SetObjectivesToVisit (- (Variables|Default|GetObjectivesToVisit) 1.0))
        (if (== (Variables|Default|GetObjectivesToVisit) 0.0)
          (bind _returnvalue (UserInterface|CreateWidget "/Game/Blueprints/WBP_WinScreen.WBP_WinScreen_C"))
          (UserInterface|Viewport|AddtoViewport _returnvalue 0))))))

(event EventTick
  (params (DeltaSeconds :type Float%20%28single-precision%29)))

(fn ConstructionScript)