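; Player controller for the MMU: drives BP_Player with six-axis movement, boost and wrist-pivot tilt, and feeds health, gas and mode to the HUD.
; Boost drains gas, which regenerates otherwise; cyclable DT_Modes rows set gas, speed and combat weights.
; A looping timer counts in-view enemies and projectiles within range, turning them into attack/defense odds.
; A weighted roll then auto-fires at an enemy, spending gas, or raises the shield.
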(event Custom|HandleHealthChanged
  (params (HealthPercent :type Float%20%28double-precision%29))
  ;[0.15 0.15 0.15 0.5] Update health
  (Default|UpdateHealth (Variables|Default|GetHUDRef) HealthPercent))

(event Input|EnhancedActionEvents|EnhancedInputActionIA_Roll
  (params (ActionValue :type Float%20%28double-precision%29) (ElapsedSeconds :type Float%20%28double-precision%29) (TriggeredSeconds :type Float%20%28double-precision%29) (InputAction :type Input%20Action%20Object%20Reference :default "/Game/Input/IA_Roll.IA_Roll"))
  ;[0.15 0.15 0.15 0.5] Roll
  (Transformation|AddActorLocalRotation (Game|Player|GetPlayerPawn 0) (Math|Rotator|MakeRotator (* ActionValue -1.0) 0.0 0.0) false false))

(event Input|EnhancedActionEvents|EnhancedInputActionIA_Mode
  (params (ActionValue :type Boolean) (ElapsedSeconds :type Float%20%28double-precision%29) (TriggeredSeconds :type Float%20%28double-precision%29) (InputAction :type Input%20Action%20Object%20Reference :default "/Game/Input/IA_Mode.IA_Mode"))
  (:Started
    (CallFunction|CycleMode)
    (CallFunction|ApplyMode)))

(event Input|EnhancedActionEvents|EnhancedInputActionIA_Boost
  (params (ActionValue :type Boolean) (ElapsedSeconds :type Float%20%28double-precision%29) (TriggeredSeconds :type Float%20%28double-precision%29) (InputAction :type Input%20Action%20Object%20Reference :default "/Game/Input/IA_Boost.IA_Boost"))
  (bind _maxgas (Variables|Default|GetMaxGas))
  ;[0.15 0.15 0.15 0.5] Boost
  (:Triggered
    (Variables|Default|SetIsBoosting true)
    (bind _output_get (Variables|Default|SetGas (Math|Float|Clamp(Float) (- (Variables|Default|GetGas) (* (Variables|Default|GetGasDrain) (Utilities|Time|GetWorldDeltaSeconds))) 0.0 _maxgas)))
    (Default|UpdateGas (Variables|Default|GetHUDRef) (/ _output_get _maxgas))
    (if (>= (Variables|Default|GetGas) 5.0)
      (Variables|Default|SetCurrentSpeed (* (Variables|Default|GetMoveSpeed) (Variables|Default|GetBoostSpeed)))
      (else
        (Variables|Default|SetCurrentSpeed (Variables|Default|GetMoveSpeed) :!label _label))))
  (:Completed
    (Variables|Default|SetIsBoosting false)
    (goto _label)))

(event Input|EnhancedActionEvents|EnhancedInputActionIA_Movement
  (params (ActionValue :type Vector :default "0, 0, 0") (ElapsedSeconds :type Float%20%28double-precision%29) (TriggeredSeconds :type Float%20%28double-precision%29) (InputAction :type Input%20Action%20Object%20Reference :default "/Game/Input/IA_Movement.IA_Movement"))
  (bind _lwrist_pivot (Variables|Default|GetLWrist_Pivot))
  (bind _relativerotation (Variables|/Script/Engine.SceneComponent|GetRelativeRotation _lwrist_pivot))
  (bind (_roll _pitch) (Math|Rotator|BreakRotator _relativerotation))
  ;[0.15 0.15 0.15 0.5] 3d Movement
  (:Triggered
    (Variables|Default|SetMovement ActionValue)
    (Transformation|AddActorWorldOffset (Game|Player|GetPlayerPawn 0) (+ (* (Math|Vector|GetForwardVector (Variables|Default|GetMMU_Pivot)) (Variables|Default|GetCurrentSpeed) (.x (Variables|Default|GetMovement))) (* (Math|Vector|GetRightVector (Variables|Default|GetMMU_Pivot)) (Variables|Default|GetCurrentSpeed) (.y (Variables|Default|GetMovement))) (* (Math|Vector|GetUpVector (Variables|Default|GetMMU_Pivot)) (Variables|Default|GetCurrentSpeed) (.z (Variables|Default|GetMovement)))) true)
    ;[0.15 0.15 0.15 0.5] Wrist rotation
    (Transformation|SetRelativeRotation _lwrist_pivot (Math|Rotator|MakeRotator (.roll (Math|Rotator|MakeRotator (Math|Float|Clamp(Float) (Math|Rotator|NormalizeAxis (+ _roll (.y (Variables|Default|GetMovement)))) -1e+01 1e+01) (Math|Float|Clamp(Float) (Math|Rotator|NormalizeAxis (+ _pitch (* (.x (Variables|Default|GetMovement)) -1.0))) -1e+01 1e+01) 0.0)) (.pitch (Math|Rotator|MakeRotator (Math|Float|Clamp(Float) (Math|Rotator|NormalizeAxis (+ _roll (.y (Variables|Default|GetMovement)))) -1e+01 1e+01) (Math|Float|Clamp(Float) (Math|Rotator|NormalizeAxis (+ _pitch (* (.x (Variables|Default|GetMovement)) -1.0))) -1e+01 1e+01) 0.0)) 0.0) false false))
  (:Completed
    (CallFunction|ResetWristRotation)))

(event Input|EnhancedActionEvents|EnhancedInputActionIA_Yaw
  (params (ActionValue :type Float%20%28double-precision%29) (ElapsedSeconds :type Float%20%28double-precision%29) (TriggeredSeconds :type Float%20%28double-precision%29) (InputAction :type Input%20Action%20Object%20Reference :default "/Game/Input/IA_Yaw.IA_Yaw"))
  ;[0.15 0.15 0.15 0.5] Mouse X Yaw
  (bind _mmu_pivot (Variables|Default|GetMMU_Pivot)
    (:then
      (Class|Actor|AddActorWorldRotation (Game|Player|GetPlayerPawn 0) (Math|Vector|RotatorfromAxisandAngle (Math|Vector|GetUpVector _mmu_pivot) ActionValue)))
    (:else)))

(event Input|EnhancedActionEvents|EnhancedInputActionIA_Pitch
  (params (ActionValue :type Float%20%28double-precision%29) (ElapsedSeconds :type Float%20%28double-precision%29) (TriggeredSeconds :type Float%20%28double-precision%29) (InputAction :type Input%20Action%20Object%20Reference :default "/Game/Input/IA_Pitch.IA_Pitch"))
  ;[0.15 0.15 0.15 0.5] Mouse Y Pitch
  (bind _mmu_pivot (Variables|Default|GetMMU_Pivot)
    (:then
      (Class|Actor|AddActorWorldRotation (Game|Player|GetPlayerPawn 0) (Math|Vector|RotatorfromAxisandAngle (* (Math|Vector|GetRightVector _mmu_pivot) "-1.000000,-1.000000,-1.000000") ActionValue)))
    (:else)))

(event EventBeginPlay
  ;[0.15 0.15 0.15 0.5] Enable Inputs
  (Input|AddMappingContext (PlayerController|LocalPlayerSubsystems|GetEnhancedInputLocalPlayerSubsystem (Game|GetPlayerController 0)) "/Game/Input/IMC_MMU.IMC_MMU" 0 "(bIgnoreAllPressedKeysUntilRelease=True,bForceImmediately=False,bNotifyUserSettings=False)")
  ;[0.15 0.15 0.15 0.5] Set MMU Pivot
  (bind _asbp_player (Utilities|Casting|CastToBP_Player (Pawn|GetControlledPawn)))
  (Variables|Default|SetMMU_Pivot (Variables|/Game/Blueprints/BP_Player.BP_Player_C|GetMMU_Pivot _asbp_player))
  ;[0.15 0.15 0.15 0.5] Set wrist pivot
  (bind _asbp_player_2 (Utilities|Casting|CastToBP_Player (Pawn|GetControlledPawn)))
  (Variables|Default|SetLWrist_Pivot (Variables|/Game/Blueprints/BP_Player.BP_Player_C|GetLWrist_Pivot _asbp_player_2))
  ;[0.15 0.15 0.15 0.5] Set ui
  (bind _returnvalue (UserInterface|CreateWidget "/Game/Blueprints/WBP_HUD.WBP_HUD_C" (Game|GetPlayerController 0)))
  (bind _output_get (Variables|Default|SetHUDRef _returnvalue))
  (UserInterface|Viewport|AddtoViewport _output_get 0)
  ;[0.15 0.15 0.15 0.5] Update health
  (EventDispatchers|BindEventtoOnHealthChanged (Variables|/Game/Blueprints/BP_Player.BP_Player_C|GetBP_HealthComponent _asbp_player_2) (delegate Custom|HandleHealthChanged))
  ;[0.15 0.15 0.15 0.5] Gas and Mode
  (CallFunction|ApplyMode)
  (Variables|Default|SetGas (Variables|Default|GetMaxGas))
  (Default|UpdateGas (Variables|Default|GetHUDRef) (/ (Variables|Default|GetGas) (Variables|Default|GetMaxGas)))
  ;[0.15 0.15 0.15 0.5] Set chance every cooldown
  (Utilities|Time|SetTimerbyFunctionName 0 "SetChance" (Variables|Default|GetCooldown) true))

(event EventTick
  (params (DeltaSeconds :type Float%20%28single-precision%29))
  (bind _hudref (Variables|Default|GetHUDRef))
  ;[0.15 0.15 0.15 0.5] Regen gas
  (if (not (Variables|Default|GetIsBoosting))
    (bind _output_get (Variables|Default|SetGas (Math|Float|Clamp(Float) (+ (Variables|Default|GetGas) (* (Variables|Default|GetGasRegen) (Utilities|Time|GetWorldDeltaSeconds))) 0.0 (Variables|Default|GetMaxGas))))
    (Utilities|IsValid _hudref
      (:Is%20Valid
        (Default|UpdateGas _hudref (/ _output_get (Variables|Default|GetMaxGas)))))))

(event Input|KeyboardEvents|H
  (params (Key :type Key%20Structure :default "None"))
  ;[0.15 0.15 0.15 0.5] Test damage
)

(fn ConstructionScript)

(fn ResetWristRotation
  (Transformation|SetRelativeRotation (Variables|Default|GetLWrist_Pivot) (Math|Rotator|MakeRotator 0.0 0.0 0.0) false false))

(fn CycleMode
  (Variables|Default|SetCurrentMode (Math|Integer|%(Integer) (+ (Variables|Default|GetCurrentMode) 1) 3))
  (CallFunction|ApplyMode))

(fn ApplyMode
  (bind _hudref (Variables|Default|GetHUDRef))
  (bind _returnvalue (Utilities|GetDataTableRow "/Game/Blueprints/DT_Modes.DT_Modes" (Utilities|String|StringToName (Utilities|String|ToString(Integer) (Variables|Default|GetCurrentMode))))
    (:then
      (Variables|Default|SetMaxGas (.maxgas _returnvalue))
      (Variables|Default|SetGasRegen (.gasregen _returnvalue))
      (Variables|Default|SetGasDrain (.gasdrain _returnvalue))
      (Variables|Default|SetMoveSpeed (.movespeed _returnvalue))
      (Variables|Default|SetGas (Math|Float|Clamp(Float) (Variables|Default|GetGas) 0.0 (Variables|Default|GetMaxGas)))
      (Default|UpdateGas _hudref (/ (Variables|Default|GetGas) (Variables|Default|GetMaxGas)))
      (Default|UpdateMode _hudref (Utilities|Text|ToText(String) (.modename _returnvalue))))))

(fn SetChance
  (bind _returnvalue (Utilities|GetDataTableRow "/Game/Blueprints/DT_Modes.DT_Modes" (Utilities|String|StringToName (Utilities|String|ToString(Integer) (Variables|Default|GetCurrentMode))))
    (:then
      (CallFunction|GetEnemiesinRange)
      (CallFunction|GetProjectilesinRange)
      (Variables|Default|SetAttackChance (Math|Float|SafeDivide (* (.shootchance _returnvalue) (Variables|Default|GetEnemiesInRange)) (+ (* (.shootchance _returnvalue) (Variables|Default|GetEnemiesInRange)) (* (+ (Variables|Default|GetProjectilesInRange) (Variables|Default|GetEnemiesInRange)) (.defensechance _returnvalue)))))
      (Variables|Default|SetDefenseChance (Math|Float|SafeDivide (* (+ (Variables|Default|GetProjectilesInRange) (Variables|Default|GetEnemiesInRange)) (.defensechance _returnvalue)) (+ (* (+ (Variables|Default|GetProjectilesInRange) (Variables|Default|GetEnemiesInRange)) (.defensechance _returnvalue)) (* (.shootchance _returnvalue) (Variables|Default|GetEnemiesInRange)))))
      (CallFunction|DoAction))))

(fn GetEnemiesinRange
  (Variables|Default|SetEnemiesInRange 0)
  (bind _outactors (Actor|GetAllActorsOfClass "/Game/Blueprints/BP_Enemy.BP_Enemy_C"))
  (for _array_element _outactors
    (bind _result (CallFunction|IsinView _array_element))
    (if (and (<= (Transformation|GetDistanceTo _array_element (Game|Player|GetPlayerPawn 0)) (Variables|Default|GetEnemyDetectRange)) _result)
      (Variables|Default|SetEnemiesInRange (+ (Variables|Default|GetEnemiesInRange) 1)))))

(fn GetProjectilesinRange
  (Variables|Default|SetProjectilesInRange 0)
  (bind _outactors (Actor|GetAllActorsOfClass "/Game/Blueprints/BP_EnemyProjectile.BP_EnemyProjectile_C"))
  (for _array_element _outactors
    (bind _result (CallFunction|IsinView _array_element))
    (if (and (<= (Transformation|GetDistanceTo _array_element (Game|Player|GetPlayerPawn 0)) (Variables|Default|GetProjectileDetectRange)) _result)
      (Variables|Default|SetProjectilesInRange (+ (Variables|Default|GetProjectilesInRange) 1)))))

(fn DoAction
  (bind _attackchance (Variables|Default|GetAttackChance))
  (bind _defensechance (Variables|Default|GetDefenseChance))
  (bind _returnvalue (+ _attackchance _defensechance))
  (bind _returnvalue_2 (Math|Random|RandomFloatinRange 0.0 _returnvalue))
  (if (not (== _returnvalue_2 0.0))
    ;[0.15 0.15 0.15 0.5] Check if you have enough gas
    (if (>= (Variables|Default|GetGas) (Variables|Default|GetActionCost))
      (if (< _returnvalue_2 (Variables|Default|GetAttackChance))
        (CallFunction|Shoot)
        ;[0.15 0.15 0.15 0.5] Disable shield
        (bind _asbp_player (Utilities|Casting|CastToBP_Player (Game|Player|GetPlayerPawn 0) :!label _label))
        (Rendering|SetVisibility (Variables|/Game/Blueprints/BP_Player.BP_Player_C|GetShield _asbp_player) false false)
        (Collision|SetCollisionEnabled (Variables|/Game/Blueprints/BP_Player.BP_Player_C|GetShieldCollider _asbp_player) "NoCollision")
        (else
          (CallFunction|Shield)))
      (else
        (goto _label)))))

(fn Shoot
  (bind _returnvalue (Game|Player|GetPlayerPawn 0))
  (bind _returnvalue_2 (Transformation|GetActorLocation _returnvalue))
  (bind _target (CallFunction|GetNearestEnemy))
  (if (Utilities|IsValid _target)
    (Game|SpawnActorfromClass "/Game/Blueprints/BP_PlayerProjectile.BP_PlayerProjectile_C" (Math|Transform|MakeTransform (+ _returnvalue_2 (* (Transformation|GetActorForwardVector _returnvalue) "200.000000,200.000000,200.000000")) (Math|Rotator|FindLookatRotation _returnvalue_2 (Transformation|GetWorldLocation (Variables|/Game/Blueprints/BP_Enemy.BP_Enemy_C|GetCube _target))) "1.000000,1.000000,1.000000") "AlwaysSpawn" "MultiplyWithRoot" _returnvalue 0)
    ;[0.15 0.15 0.15 0.5] Reduce gas per shot
    (CallFunction|ReduceGas (Variables|Default|GetShootCost))))

(fn Shield
  (bind _asbp_player (Utilities|Casting|CastToBP_Player (Game|Player|GetPlayerPawn 0)))
  (Rendering|SetVisibility (Variables|/Game/Blueprints/BP_Player.BP_Player_C|GetShield _asbp_player) true false)
  (Collision|SetCollisionEnabled (Variables|/Game/Blueprints/BP_Player.BP_Player_C|GetShieldCollider _asbp_player) "QueryAndPhysics"))

(fn IsinView
  (params (Enemy :type Actor%20Object%20Reference))
  (bind _returnvalue (Game|GetPlayerCameraManager 0))
  (return (>= (Math|Vector|DotProduct (Math|Vector|GetForwardVector (Camera|GetCameraRotation _returnvalue)) (Math|Vector|GetUnitDirection(Vector) (Camera|GetCameraLocation _returnvalue) (Transformation|GetActorLocation Enemy))) (Math|Trig|Cos(Degrees) (/ (Variables|Default|GetViewAngle) 2.0)))))

(fn ReduceGas
  (params (Amount :type Float%20%28double-precision%29))
  (Variables|Default|SetGas (Math|Float|Clamp(Float) (- (Variables|Default|GetGas) Amount) 0.0 (Variables|Default|GetMaxGas))))

(fn GetNearestEnemy
  (bind _outactors (Actor|GetAllActorsOfClass "/Game/Blueprints/BP_Enemy.BP_Enemy_C"))
  (for _array_element _outactors
    (if (and (< (Transformation|GetDistanceTo _array_element (Game|Player|GetPlayerPawn 0)) (LocalVariables|GetBestDist)) (<= (Transformation|GetDistanceTo _array_element (Game|Player|GetPlayerPawn 0)) (Variables|Default|GetEnemyDetectRange)))
      (LocalVariables|SetBestDist (Transformation|GetDistanceTo _array_element (Game|Player|GetPlayerPawn 0)))
      (LocalVariables|SetBest _array_element)
      (return (LocalVariables|GetBest)))))